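; BP_ArenaCenter is an arena center zone that boosts player characters while they are inside its sphere.
; When a BP_Character begins overlapping the sphere, it sets IsInArea and calls StartBoosting on that character's BP_PlayerState.
; Ending the overlap clears the flag and calls StopBoosting, leaving the boost logic to the player state.
; IsInArea is a single flag shared by all characters, and both transitions print debug messages.
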(event `self.Sphere.OnComponentBeginOverlap`
  (params (OverlappedComponent :type "PrimitiveComponent Object Reference") (OtherActor :type "Actor Object Reference") (OtherComp :type "PrimitiveComponent Object Reference") (OtherBodyIndex :type Integer) (bFromSweep :type Boolean) (SweepResult :type "HitResult Structure (by ref)"))
  (bind _asbp_character (cast `/Game/MyContent/Characters/BP_Character` OtherActor))
  (set `self.IsInArea` true)
  (bind _asbp_player_state (cast `/Game/MyContent/Player/BP_PlayerState` (`Pawn.PlayerState` _asbp_character)))
  (`/Game/MyContent/Player/BP_PlayerState.Start boosting` _asbp_player_state)
  (`KismetSystemLibrary.PrintString` "boosing"))

(event `self.Sphere.OnComponentEndOverlap`
  (params (OverlappedComponent :type "PrimitiveComponent Object Reference") (OtherActor :type "Actor Object Reference") (OtherComp :type "PrimitiveComponent Object Reference") (OtherBodyIndex :type Integer))
  (`/Engine/EditorBlueprintResources/StandardMacros.IsValid` OtherActor
    (:`Is Valid`
      (bind _asbp_character (cast `/Game/MyContent/Characters/BP_Character` OtherActor))
      (set `self.IsInArea` false)
      (bind _asbp_player_state (cast `/Game/MyContent/Player/BP_PlayerState` (`Pawn.PlayerState` _asbp_character)))
      (`/Game/MyContent/Player/BP_PlayerState.Stop Boosting` _asbp_player_state)
      (`KismetSystemLibrary.PrintString` "not boosting"))))

(fn `UserConstructionScript`)