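; BP_UpgradeWeapon is an upgrade zone that grants a timed weapon upgrade, labelled as shotgun, to a BP_Character standing in its sphere.
; On the server, entering the sphere calls UpgradeWeaponAfterTime on the character and leaving calls EndShotgunTimer.
; Ten seconds after entry, the server deactivates the upgrade effect and sphere components and hides the spotlight.
; The UpgradeWeapon event is empty, and several leftover node chains never run.
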(event `self.ReceiveBeginPlay`)

(event `self.Sphere.OnComponentBeginOverlap`
  (params (OverlappedComponent :type "PrimitiveComponent Object Reference") (OtherActor :type "Actor Object Reference") (OtherComp :type "PrimitiveComponent Object Reference") (OtherBodyIndex :type Integer) (bFromSweep :type Boolean) (SweepResult :type "HitResult Structure (by ref)"))
  (bind _asbp_character (cast `/Game/MyContent/Characters/BP_Character` OtherActor))
  (`/Engine/EditorBlueprintResources/ActorMacros.Switch Has Authority`
    (:`Authority`
      (`/Game/MyContent/Characters/BP_Character.UpgradeWeaponAfterTime` _asbp_character (`self.UpgradeTime`))
      (`KismetSystemLibrary.PrintString` "upgrade to SHOTGUN" true true (struct :`R` 1.0 :`G` 0.920566 :`B` 0.201985 :`A` 1.0))
      (if true
        (`KismetSystemLibrary.Delay` 10.0)
        (`ActorComponent.Deactivate` (`self.NS_UpgradeWeapon`))
        (`ActorComponent.Deactivate` (`self.Sphere`))
        (`SceneComponent.SetVisibility` (`self.SpotLight`) false false)))))

(event `self.Sphere.OnComponentEndOverlap`
  (params (OverlappedComponent :type "PrimitiveComponent Object Reference") (OtherActor :type "Actor Object Reference") (OtherComp :type "PrimitiveComponent Object Reference") (OtherBodyIndex :type Integer))
  (bind _asbp_character (cast `/Game/MyContent/Characters/BP_Character` OtherActor))
  (`/Engine/EditorBlueprintResources/ActorMacros.Switch Has Authority`
    (:`Authority`
      (`/Game/MyContent/Characters/BP_Character.EndShotgunTimer` _asbp_character))))

(event `UpgradeWeapon`
  (params (PlayerIndex :type Integer)))

(fn `UserConstructionScript`)