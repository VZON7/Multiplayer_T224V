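; Lobby game mode that gives each joining player a numbered default name.
; On PostLogin it casts the player's state to BP_PlayerState and sets the name to "Player" plus the current player state count.
; An unconnected branch, which never runs, would restart a player at the PlayerStart tagged for their join number, covering up to four players.
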(event `self.K2_PostLogin`
  (params (NewPlayer :type "PlayerController Object Reference"))
  (bind _asbp_player_state (cast `/Game/MyContent/Player/BP_PlayerState` (`Controller.PlayerState` NewPlayer)))
  (`/Game/MyContent/Player/BP_PlayerState.SetPlayerName` _asbp_player_state (`KismetStringLibrary.Concat_StrStr` "Player " (`KismetStringLibrary.Conv_IntToString` (`GameplayStatics.GetNumPlayerStates`)))))

(fn `UserConstructionScript`)