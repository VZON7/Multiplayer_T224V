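; BP_Pickup_Weapon is a pickup that gives a character the weapon defined by its WeaponAsset.
; The construction script shows that asset's skeletal mesh, and Pickup calls ActivateWeapon on the character with the asset's weapon class.
; Deactivate and reactivate overrides call the parent, then hide or show the mesh.
; The event graph holds only disabled stub events.
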(fn `OnDeactivate`
  (`parent.OnDeactivate`)
  (`SceneComponent.SetVisibility` (`self.SkeletalMesh`) false false))

(fn `OnReactivate`
  (`parent.OnReactivate`)
  (`SceneComponent.SetVisibility` (`self.SkeletalMesh`) true false))

(fn `Pickup`
  (params (Character :type "/Game/MyContent/Characters/BP_Character Object Reference"))
  (bind _weaponasset (`self.WeaponAsset`)
    (:`then`
      (`/Game/MyContent/Characters/BP_Character.ActivateWeapon` Character (`/Game/MyContent/PickUp/BP_DA_WeaponPickup.WeaponClass` _weaponasset)))
    (:`else`)))

(fn `UserConstructionScript`
  (`parent.UserConstructionScript`)
  (bind _weaponasset (`self.WeaponAsset`)
    (:`then`
      (`SkeletalMeshComponent.SetSkeletalMeshAsset` (`self.SkeletalMesh`) (`/Game/MyContent/PickUp/BP_DA_WeaponPickup.SkeletalMesh` _weaponasset)))
    (:`else`)))