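; Shotgun weapon Blueprint that fires several line-damage pellets per shot, built on a parent weapon class.
; On BeginPlay it divides Damage by BulletPerShot, splitting one shot's damage across the pellets.
; ActivateDamage calls ApplyLineDamage per pellet, picking random directions in cones that widen with the pellet index, so the first goes straight and later ones can stray further.
; Each trace requests timed debug drawing.
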(event `self.ReceiveBeginPlay`
  (set `self.Damage` (/ (`self.Damage`) (`self.BulletPerShot`))))

(fn `ActivateDamage`
  (params (ShootLoc :type "Vector Structure") (ShootDir :type "Vector Structure"))
  (bind _bulletpershot (`self.BulletPerShot`))
  (for _index (range _bulletpershot)
    (`self.ApplyLineDamage` (`local.ShootLoc`) (`KismetMathLibrary.RandomUnitVectorInConeInDegrees` (`local.ShootDir`) (* _index (/ (`self.SpreadAngle`) _bulletpershot))) "ForDuration")))

(fn `UserConstructionScript`
  (`parent.UserConstructionScript`))